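; BP_Statue is a collectible statue that jumps to random spots in the level until the player touches it.
; On BeginPlay it caches BP_Guide_GameMode and runs InitStatue, which teleports it within a fixed area at constant height and re-arms itself by timer, with shorter intervals at higher levels.
; Player overlap before game over calls StatueCollected on the game mode, destroys the statue and spawns a replacement.
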(event EventBeginPlay
  (bind _asbp_guide_game_mode (Utilities|Casting|CastToBP_Guide_GameMode (Game|GetGameMode)))
  (Variables|Default|SetAs%20BP%20Guide%20Game%20Mode _asbp_guide_game_mode)
  (CallFunction|InitStatue))

(event Collision|EventActorBeginOverlap
  (params (OtherActor :type Actor%20Object%20Reference))
  (bind _as_bp_guide_game_mode (Variables|Default|GetAs%20BP%20Guide%20Game%20Mode))
  (if (and (== OtherActor (Game|GetPlayerCharacter 0)) (not (Variables|/Game/Custom_Blueprints/BP_Guide_GameMode.BP_Guide_GameMode_C|GetGameOver _as_bp_guide_game_mode)))
    (Default|StatueCollected _as_bp_guide_game_mode)
    (Actor|DestroyActor)
    (Game|SpawnActorfromClass "BP_Statue_C" (Transformation|GetActorTransform) "Undefined" 0 0)))

(fn ConstructionScript)

(fn InitStatue
  (Transformation|Teleport (Math|Vector|MakeVector (Math|Random|RandomFloatinRange -1.8e+03 1e+03) (Math|Random|RandomFloatinRange -1.4e+03 1.4e+03) 1.3e+02) "0, 0, 0")
  (Utilities|Time|SetTimerbyFunctionName 0 "InitStatue" (Math|Conversions|ToFloat(Integer) (- 6 (Variables|/Game/Custom_Blueprints/BP_Guide_GameMode.BP_Guide_GameMode_C|GetLevel (Variables|Default|GetAs%20BP%20Guide%20Game%20Mode))))))